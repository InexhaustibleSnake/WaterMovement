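; Main character Blueprint that adds swimming and depth-based movement slowdown in Flux fluid water.
; Each tick, mesh depth below the Flux surface remaps MaxWalkSpeed from the current max speed toward a fixed underwater value.
; The upward axis feeds the BPFluxSwimming component, while the downward axis applies vertical movement input directly.
; Ragdoll, modifier and interaction functions are empty stubs.
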(event EventTick
  (params (DeltaSeconds :type Float%20%28single-precision%29))
  ;[1 1 1] Event Tick
  (|CallParentFunction DeltaSeconds)
  (CallFunction|UnderWaterMovement))

(event Input|AxisEvents|InputAxisSwimDown
  (params (AxisValue :type Float%20%28single-precision%29))
  ;[1 1 1] Swim Down
  (Pawn|Input|AddMovementInput (Math|Vector|MakeVector 0.0 0.0 AxisValue) (Variables|Default|GetSwimZSpeed) false))

(event Input|AxisEvents|InputAxisSwimUpward
  (params (AxisValue :type Float%20%28single-precision%29))
  ;[1 1 1] Swim Upward
  (Variables|/Game/FluidFlux/Environment/Swimming/BP_FluxSwimmingComponent.BP_FluxSwimmingComponent_C|SetInputSwimUp (Variables|Default|GetBP_FluxSwimming) AxisValue))

(fn ConstructionScript
  (|CallParentFunction))

(fn UpdateRagdoll
  (params (A :type Float%20%28double-precision%29)))

(fn UnderWaterMovement
  (Variables|Default|SetDepth (- (.z (Variables|/Game/FluidFlux/Environment/Readback/BP_FluxDataComponent.BP_FluxDataComponent_C|GetFluxSurfaceLocation (Variables|Default|GetBP_FluxDataComponent))) (.z (Transformation|GetWorldLocation (Variables|Character|GetMesh)))))
  (Variables|/Script/Engine.CharacterMovementComponent|SetMaxWalkSpeed (Variables|Character|GetCharacterMovement) (Math|Float|MapRangeClamped (Variables|Default|GetDepth) 4e+01 2e+02 (Class|MovementComponent|GetMaxSpeed (Variables|Character|GetCharacterMovement)) 2.4e+02)))

(fn AddModifiers
  (params (Modifiers :type Array%20of%20BP%20Flux%20Modifier%20Component%20Object%20References))
  (return false))

(fn GetInteractions
  (params (Ratio :type Float%20%28double-precision%29) (Iteration :type Integer))
  (return 0))

(fn IgnoreModifierOverlap
  (params (Copmponent :type Actor%20Component%20Object%20Reference))
  (return false))